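; BP_AVP2_Mirror_05 is a mirror prop from an ArchVis asset pack with adjustable surface appearance.
; Its construction script creates a dynamic instance of M_AVP2_Mirrors on element 0 of the static mesh, assigning the base color, mask and normal textures.
; It then feeds the Blueprint's metalness, roughness and color variables into that material, while the event graph holds only disabled placeholder events.
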(fn `UserConstructionScript`
  (bind _returnvalue (`PrimitiveComponent.CreateDynamicMaterialInstance` (`self.StaticMesh`) 0 "/Game/Assets/3D_Assets/ArchVisPolishPack02/Materials/M_AVP2_Mirrors.M_AVP2_Mirrors" "None"))
  (`MaterialInstanceDynamic.SetTextureParameterValue` _returnvalue "Base Color Texture" "/Game/Assets/3D_Assets/ArchVisPolishPack02/Textures/T_AVP2_Mirrors_D.T_AVP2_Mirrors_D")
  (`MaterialInstanceDynamic.SetTextureParameterValue` _returnvalue "Mask Texture" "/Game/Assets/3D_Assets/ArchVisPolishPack02/Textures/T_AVP2_Mirrors_M.T_AVP2_Mirrors_M")
  (`MaterialInstanceDynamic.SetTextureParameterValue` _returnvalue "Normal Texture" "/Game/Assets/3D_Assets/ArchVisPolishPack02/Textures/T_AVP2_Mirrors_N.T_AVP2_Mirrors_N")
  (`MaterialInstanceDynamic.SetScalarParameterValue` _returnvalue "Mirrors.Metalness" (`self.Mirrors.Metalness`))
  (`MaterialInstanceDynamic.SetScalarParameterValue` _returnvalue "Mirrors.Roughness" (`self.Mirrors.Roughness`))
  (`MaterialInstanceDynamic.SetVectorParameterValue` _returnvalue "Mirrors.Color" (`self.Mirrors.Color`)))