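; BP_AVP2_Deco_Glass_06 is a glass decoration prop from the ArchVis Polish Pack with an adjustable glass look.
; Its Construction Script creates a dynamic instance of M_AVP2_Glass on the static mesh's first material slot.
; It then feeds the Blueprint's opacity, roughness, color and two refraction variables into the matching material parameters.
; The event graph holds only disabled placeholder events, so no gameplay logic runs.
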(fn `UserConstructionScript`
  (bind _returnvalue (`PrimitiveComponent.CreateDynamicMaterialInstance` (`self.StaticMesh`) 0 "/Game/3D_Assets/ArchVisPolishPack02/Materials/M_AVP2_Glass.M_AVP2_Glass" "None"))
  (`MaterialInstanceDynamic.SetScalarParameterValue` _returnvalue "Glass.Opacity" (`self.Glass.Opacity`))
  (`MaterialInstanceDynamic.SetScalarParameterValue` _returnvalue "Glass.Roughness" (`self.Glass.Roughness`))
  (`MaterialInstanceDynamic.SetVectorParameterValue` _returnvalue "Glass.Color" (`self.Glass.Color`))
  (`MaterialInstanceDynamic.SetScalarParameterValue` _returnvalue "Glass.RefractionA" (`self.Glass.RefractionA`))
  (`MaterialInstanceDynamic.SetScalarParameterValue` _returnvalue "Glass.RefractionB" (`self.Glass.RefractionB`)))