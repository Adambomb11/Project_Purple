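; Quicksand block that turns to glass and then prompts the purple player character to interact with it.
; When a BP_Barrel overlaps the mesh while Red's ability is active, it swaps to a glass material, plays a hit sound and becomes purple-interactable.
; A sphere trigger tracks purple proximity.
; Tick shows the use prompt, with a gamepad or keyboard icon; the interaction itself is not handled here.
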(event `self.ReceiveBeginPlay`
  (bind _asblue_als_anim_man_character_bp (cast `/Game/AdvancedLocomotionV4/Blueprints/CharacterLogic/BLUE_ALS_AnimMan_CharacterBP` (`GameplayStatics.GetPlayerCharacter` 0)))
  (bind _output_get (set `self.Player BLUE` _asblue_als_anim_man_character_bp)))

(event `self.ReceiveTick`
  (params (DeltaSeconds :type "Float (single-precision)"))
  (bind _pressfwidget (`self.PressFWidget`))
  (bind _isplayernear (`self.IsPlayerNear`))
  (bind _returnvalue (and (`self.PurpleInteractable`) (`self.IsPlayerNear`) (`self.isGlassBlock`)))
  (if _returnvalue
    (if _isplayernear
      (`SceneComponent.SetVisibility` _pressfwidget _isplayernear false)
      (bind _aswbp_use_purple (cast `/Game/UI/WBP/WBP_Use_Purple` (`WidgetComponent.GetWidget` _pressfwidget)))
      (`Image.SetBrushFromTexture` (`/Game/UI/WBP/WBP_Use_Purple.Control` _aswbp_use_purple) (select `bool` (`/Game/AdvancedLocomotionV4/Blueprints/CharacterLogic/BLUE_ALS_AnimMan_CharacterBP.GamepadOn` (stale `self.ReceiveBeginPlay` _output_get)) :`false` "/Game/UI/Assets/Input_Icons/Keyboard___Mouse/Light/F_Key_Light.F_Key_Light" :`true` "/Game/UI/Assets/Input_Icons/Others/Xbox_One/XboxOne_X.XboxOne_X" :!type "Texture2D Object Reference") false))
    (else
      (`SceneComponent.SetVisibility` (`self.PressFWidget`) _returnvalue false))))

(event `self.Mesh.OnComponentBeginOverlap`
  (params (OverlappedComponent :type "PrimitiveComponent Object Reference") (OtherActor :type "Actor Object Reference") (OtherComp :type "PrimitiveComponent Object Reference") (OtherBodyIndex :type Integer) (bFromSweep :type Boolean) (SweepResult :type "HitResult Structure (by ref)"))
  (if (`self.isGlassBlock`)
    ;[0 1 0.1029] Turning Sand to glass
    (if (`/Game/AdvancedLocomotionV4/Blueprints/CharacterLogic/BLUE_ALS_AnimMan_CharacterBP.IsPurple` (`self.Player BLUE`))
      (set `self.PurpleInteractable` true :!label _label))
    (else
      (bind _player_blue (`self.Player BLUE`)
        (:`then`
          (if (`/Game/AdvancedLocomotionV4/Blueprints/CharacterLogic/RED_ALS_AnimMan_CharacterBP.Red_Ability` (`/Game/AdvancedLocomotionV4/Blueprints/CharacterLogic/BLUE_ALS_Base_CharacterBP.Player_Red` _player_blue))
            (cast `/Game/AdvancedLocomotionV4/Blueprints/Props/BP_Barrel` OtherActor)
            (`PrimitiveComponent.SetMaterial` (`self.Mesh`) 0 "/Game/Assets/3D_Assets/ArchVisPolishPack02/Materials/M_AVP2_Glass.M_AVP2_Glass")
            (set `self.isGlassBlock` true)
            (`GameplayStatics.PlaySound2D` "/Game/StarterContent/Maps/Hammer_Hit.Hammer_Hit" 1.0 1.0 0.0 null null)
            (goto _label)))
        (:`else`)))))

(event `self.Sphere.OnComponentBeginOverlap`
  (params (OverlappedComponent :type "PrimitiveComponent Object Reference") (OtherActor :type "Actor Object Reference") (OtherComp :type "PrimitiveComponent Object Reference") (OtherBodyIndex :type Integer) (bFromSweep :type Boolean) (SweepResult :type "HitResult Structure (by ref)"))
  ;[1 0 0.6967] Player in range (purple in range)
  (bind _asblue_als_anim_man_character_bp (cast `/Game/AdvancedLocomotionV4/Blueprints/CharacterLogic/BLUE_ALS_AnimMan_CharacterBP` OtherActor))
  (if (`/Game/AdvancedLocomotionV4/Blueprints/CharacterLogic/BLUE_ALS_AnimMan_CharacterBP.IsPurple` _asblue_als_anim_man_character_bp)
    (set `self.IsPlayerNear` true)
    (else
      (set `self.IsPlayerNear` false))))

(event `self.Sphere.OnComponentEndOverlap`
  (params (OverlappedComponent :type "PrimitiveComponent Object Reference") (OtherActor :type "Actor Object Reference") (OtherComp :type "PrimitiveComponent Object Reference") (OtherBodyIndex :type Integer))
  (bind _asblue_als_anim_man_character_bp (cast `/Game/AdvancedLocomotionV4/Blueprints/CharacterLogic/BLUE_ALS_AnimMan_CharacterBP` OtherActor))
  (if (and (`/Game/AdvancedLocomotionV4/Blueprints/CharacterLogic/BLUE_ALS_AnimMan_CharacterBP.IsPurple` _asblue_als_anim_man_character_bp) (`self.isGlassBlock`))
    (set `self.PurpleInteractable` false)
    (set `self.IsPlayerNear` false)))

(fn `UserConstructionScript`)